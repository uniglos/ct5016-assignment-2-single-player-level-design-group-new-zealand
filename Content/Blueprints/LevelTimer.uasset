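; LevelTimer is a Blueprint that records how long each level takes and persists it in a TimerSave save game.
; BeginPlay stores the start time; LevelOver writes the elapsed minutes:seconds:milliseconds string into a LevelTimes map keyed by level name in slot "DemoTime".
; The existence check queries "DemoSave" instead, so "DemoTime" is overwritten with an empty save whenever "DemoSave" is absent.
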(event Custom|LevelOver
  (bind _returnvalue (Math|DateTime|Now))
  (bind _starttime (Variables|Default|GetStartTime))
  (bind _returnvalue_2 (- _returnvalue _starttime))
  (bind _returnvalue_3 (SaveGame|DoesSaveGameExist "DemoSave"))
  (if _returnvalue_3
    _
    (else
      (bind _returnvalue_4 (SaveGame|CreateSaveGameObject "/Game/Blueprints/TimerSave.TimerSave_C"))
      (SaveGame|SaveGametoSlot _returnvalue_4 "DemoTime")))
  (bind _returnvalue_5 (SaveGame|LoadGamefromSlot "DemoTime"))
  (bind _astimer_save (Utilities|Casting|CastToTimerSave _returnvalue_5))
  (bind _returnvalue_6 (Game|GetCurrentLevelName true))
  (Utilities|Map|Add (Variables|/Game/Blueprints/TimerSave.TimerSave_C|GetLevelTimes _astimer_save) _returnvalue_6 (Utilities|String|Append (Utilities|String|ToString(Integer) (Math|Timespan|GetMinutes _returnvalue_2)) ":" (Utilities|String|ToString(Integer) (Math|Timespan|GetSeconds _returnvalue_2)) ":" (Utilities|String|ToString(Integer) (Class|KismetMathLibrary|GetMilliseconds _returnvalue_2))))
  (SaveGame|SaveGametoSlot _astimer_save "DemoTime"))

(event EventBeginPlay
  (Variables|Default|SetStartTime (Math|DateTime|Now)))

(fn ConstructionScript)
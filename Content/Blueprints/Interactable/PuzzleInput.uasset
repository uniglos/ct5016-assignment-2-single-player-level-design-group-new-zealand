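; Interactable puzzle input that cycles through a list of symbols, showing the current one on a decal beside a coloured button.
; Each interaction advances the wrapping index, fires OnUpdate and swaps the icon texture on a dynamic decal material.
; SelectionCorrect locks the input by unbinding interaction and turns the decal green.
; SetupHint passes a given symbol, the input's colour and a number to its Hint and sets the number text.
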(event Custom|ChangeSelection
  (bind _result (Math|Integer|IncrementInt (Variables|Default|GetValue))
    (:%20%20
      (if (< _result (Utilities|Array|Length (Variables|Default|GetSymbols)))
        _
        (else
          (Variables|Default|SetValue 0)))
      (Default|CallOnUpdate)
      (CallFunction|DisplaySelection))))

(event Custom|SelectionCorrect
  (EventDispatchers|UnbindEventfromOnInteraction (Variables|Default|GetInteractTriggerComponent) (delegate Custom|ChangeSelection))
  (Rendering|Components|Decal|SetDecalColor (Variables|Default|GetDecal) (Utilities|Struct|MakeLinearColor 0.0 1.0 0.0 1.0)))

(event Custom|SetButtonColour
  (params (Colour :type Linear%20Color%20Structure))
  (bind _returnvalue (Rendering|Material|CreateDynamicMaterialInstance (Variables|Default|GetButton) 0 0 "None" :!class /Script/Engine.PrimitiveComponent))
  (Rendering|Material|SetVectorParameterValue _returnvalue "BaseColor" Colour :!class /Script/Engine.MaterialInstanceDynamic))

(event Custom|SetupHint
  (params (Value :type Integer) (Number :type Text))
  (Rendering|Components|TextRender|SetText (Variables|Default|GetNumber) Number)
  (Default|Setup (Variables|Default|GetHint) (Utilities|Array|Get(acopy) (Variables|Default|GetSymbols) Value) (Variables|Default|GetColour) Number))

(event EventBeginPlay
  (EventDispatchers|BindEventtoOnInteraction (Variables|Default|GetInteractTriggerComponent) (delegate Custom|ChangeSelection))
  (CallFunction|DisplaySelection))

(fn ConstructionScript
  (bind _returnvalue (Rendering|Material|CreateDynamicMaterialInstance (Variables|Default|GetDecal) :!class /Script/Engine.DecalComponent))
  (Variables|Default|SetDecalMaterial _returnvalue)
  (CallFunction|SetButtonColour (Variables|Default|GetColour)))

(fn DisplaySelection
  (Rendering|Material|SetTextureParameterValue (Variables|Default|GetDecalMaterial) "PuzzleIcon" (Utilities|Array|Get(acopy) (Variables|Default|GetSymbols) (Variables|Default|GetValue))))
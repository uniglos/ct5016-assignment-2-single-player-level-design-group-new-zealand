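; A pushable physics object that responds to pushes only on its enabled X or Y axes and falls when unsupported.
; Each tick a box trace at FloorPos toggles gravity, re-enabling physics simulation when falling starts or stops.
; Allowed pushes go to the parent collision logic unless the object is falling.
; BP_Player mantle events pause tick and physics, storing the physics state, updated by pushes meanwhile, to restore afterwards.
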(event Custom|PlayerEndMantle
  (Actor|Tick|SetActorTickEnabled true)
  (Physics|SetSimulatePhysics (Variables|Default|GetStaticMeshComponent) (Variables|Default|GetMantleState)))

(event Custom|PlayerMantle
  (bind _staticmeshcomponent (Variables|Default|GetStaticMeshComponent))
  (Actor|Tick|SetActorTickEnabled false)
  (Variables|Default|SetMantleState (Physics|IsSimulatingPhysics _staticmeshcomponent "None"))
  (Physics|SetSimulatePhysics _staticmeshcomponent false))

(event EventTick
  (params (DeltaSeconds :type Float%20%28single-precision%29))
  (bind _falling (CallFunction|FloorCheck))
  (Physics|SetEnableGravity (Variables|Default|GetStaticMeshComponent) _falling)
  (if _falling
    (if (not (Variables|Default|GetPreviouslyFalling))
      (Physics|SetSimulatePhysics (Variables|Default|GetStaticMeshComponent) true))
    (elif (not (Variables|Default|GetPreviouslyFalling))
      _
      (else
        (Physics|SetSimulatePhysics (Variables|Default|GetStaticMeshComponent) true))))
  (Variables|Default|SetPreviouslyFalling _falling))

(event EventBeginPlay
  (bind _returnvalue (Actor|GetActorOfClass "/Game/Blueprints/BP_Player.BP_Player_C"))
  (EventDispatchers|BindEventtoMantleStarted _returnvalue (delegate Custom|PlayerMantle))
  (EventDispatchers|BindEventtoMantleEnded _returnvalue (delegate Custom|PlayerEndMantle)))

(fn ConstructionScript
  (|CallParentFunction))

(fn CollisionFunction
  (params (HitActor :type Actor%20Object%20Reference) (Axis :type Boolean) (Push :type Boolean))
  ;[1 1 1] If 'Axis' is 1 (indicating  Y axis), only do behaviour if the parameter 'YMove' is true.
  ; If 'Axis' is 0 (X axis), the same with 'XMove'.
  (if (or (and Axis (Variables|Default|GetYMove)) (and (not Axis) (Variables|Default|GetXMove)))
    ;[1 1 1] Additionally checks whether the object is falling, as to not interrupt it.
    (if (not (Class|PrimitiveComponent|IsGravityEnabled (Variables|Default|GetStaticMeshComponent)))
      (if (Class|Actor|IsActorTickEnabled)
        (|CallParentFunction HitActor false Push)
        (else
          (Variables|Default|SetMantleState Push))))))

(fn FloorCheck
  (bind _floorpos (Variables|Default|GetFloorPos))
  (bind _returnvalue (Transformation|GetWorldLocation _floorpos))
  (bind _returnvalue_2 (Collision|BoxTraceByChannel _returnvalue _returnvalue "100.000000,100.000000,2.500000" "0, 0, 0" "TraceTypeQuery1" false 0 "ForOneFrame"))
  (return (not _returnvalue_2)))
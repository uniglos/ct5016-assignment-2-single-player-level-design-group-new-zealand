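; A locked door that opens by moving along its local Z axis once enough linked lights are turned on.
; BeginPlay binds each entry in Lights to handlers that raise or lower an Inputs counter, and sets the timeline's play rate from Speed.
; When the count reaches the number of lights, the DoorOpen timeline plays, adding a Height-scaled offset each update.
; Turning a light off only lowers the count, with no closing logic.
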(event Custom|OpenDoor
  (bind _dooropen (Timeline|DoorOpen Play)
    (:Update
      (Transformation|AddActorLocalOffset (Math|Vector|MakeVector 0.0 0.0 (* _dooropen (Variables|Default|GetHeight))) false false))))

(event Custom|LightActivated
  (bind _result (Math|Integer|IncrementInt (Variables|Default|GetInputs))
    (:%20%20
      (if (>= _result (Utilities|Array|Length (Variables|Default|GetLights)))
        (CallFunction|OpenDoor)))))

(event Custom|LightDeactivated
  (Math|Integer|DecrementInt (Variables|Default|GetInputs)))

(event EventBeginPlay
  (for _array_element (Variables|Default|GetLights)
    (EventDispatchers|AssignTurnedOff _array_element (delegate Custom|LightDeactivated))
    (EventDispatchers|BindEventtoTurnedon _array_element (delegate Custom|LightActivated))
    (Components|Timeline|SetPlayRate (Variables|Default|GetDoorOpen) (Variables|Default|GetSpeed))))

(fn ConstructionScript)
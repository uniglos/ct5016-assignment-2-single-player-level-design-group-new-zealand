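; SymbolPuzzleMaster is an interactable puzzle controller that opens a door when its four symbol inputs show the correct combination.
; The construction script gathers the PuzzleInput actors from four child actor components into an array.
; On BeginPlay it binds to each input's update event.
; Each update compares every value with the Order array by index, and a full match opens the Door and notifies all inputs of success.
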(event Custom|InputChanged
  (bind _correct (CallFunction|CheckOrder))
  (if _correct
    (Default|OpenDoor (Variables|Default|GetDoor))
    (for _array_element (Variables|Default|GetInputObjects)
      (Default|SelectionCorrect _array_element))))

(event EventBeginPlay
  (for _array_element (Variables|Default|GetInputObjects)
    (EventDispatchers|BindEventtoOnUpdate _array_element (delegate Custom|InputChanged))))

(fn ConstructionScript
  (for _array_element (Utilities|Array|MakeArray (Variables|Default|GetPuzzleInput1) (Variables|Default|GetPuzzleInput2) (Variables|Default|GetPuzzleInput3) (Variables|Default|GetPuzzleInput4))
    (bind _aspuzzle_input (Utilities|Casting|CastToPuzzleInput (Variables|/Script/Engine.ChildActorComponent|GetChildActor _array_element)))
    (Utilities|Array|Add (Variables|Default|GetInputObjects) _aspuzzle_input)))

(fn CheckOrder
  (LocalVariables|SetPuzzleCorrect true)
  (for (_array_element _array_index) (Variables|Default|GetInputObjects)
    (if (!= (Variables|/Game/Blueprints/Interactable/PuzzleInput.PuzzleInput_C|GetValue _array_element) (Utilities|Array|Get(acopy) (Variables|Default|GetOrder) _array_index))
      (LocalVariables|SetPuzzleCorrect false)))
  (return (LocalVariables|GetPuzzleCorrect)))
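; PuzzleLight is an interactable indicator light for puzzles that toggles between a green on state and a red off state.
; The construction script creates a dynamic material instance on its Sphere.
; LightOn and LightOff recolor that material's background and glow parameters, guarded by a State flag so each fires only on a change, and call TurnedOn or TurnedOff to signal the switch.
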(event Custom|LightOn
  (bind _lightmaterial (Variables|Default|GetLightMaterial))
  (if (not (Variables|Default|GetState))
    (Rendering|Material|SetVectorParameterValue _lightmaterial "ColorBG" "(R=0.000000,G=1.000000,B=0.000000,A=1.000000)" :!class /Script/Engine.MaterialInstanceDynamic)
    (Rendering|Material|SetVectorParameterValue _lightmaterial "ColorGlow" "(R=0.000000,G=1.000000,B=0.000000,A=1.000000)" :!class /Script/Engine.MaterialInstanceDynamic)
    (Default|CallTurnedon)
    (Variables|Default|SetState true)))

(event Custom|LightOff
  (bind _lightmaterial (Variables|Default|GetLightMaterial))
  (if (Variables|Default|GetState)
    (Rendering|Material|SetVectorParameterValue _lightmaterial "ColorBG" "(R=1.000000,G=0.000000,B=0.000000,A=1.000000)" :!class /Script/Engine.MaterialInstanceDynamic)
    (Rendering|Material|SetVectorParameterValue _lightmaterial "ColorGlow" "(R=1.000000,G=0.000000,B=0.000000,A=1.000000)" :!class /Script/Engine.MaterialInstanceDynamic)
    (Default|CallTurnedOff)
    (Variables|Default|SetState false)))

(fn ConstructionScript
  (bind _returnvalue (Rendering|Material|CreateDynamicMaterialInstance (Variables|Default|GetSphere) 0 0 "None" :!class /Script/Engine.PrimitiveComponent))
  (Variables|Default|SetLightMaterial _returnvalue))
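; PuzzleInput is an interactable puzzle dial that cycles through a set of symbols shown on a decal.
; Each interaction reported by its InteractTriggerComponent increments Value, with a check against the Symbols array length to wrap back to zero.
; DisplaySelection applies the material at that index to the decal, both at BeginPlay and after every change.
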(event Custom|ChangeSelection
  (bind _result (Math|Integer|IncrementInt (Variables|Default|GetValue))
    (:%20%20
      (if (< _result (Utilities|Array|Length (Variables|Default|GetSymbols)))
        _
        (else
          (Variables|Default|SetValue 0)))
      (CallFunction|DisplaySelection))))

(event EventBeginPlay
  (EventDispatchers|BindEventtoOnInteraction (Variables|Default|GetInteractTriggerComponent) (delegate Custom|ChangeSelection))
  (CallFunction|DisplaySelection))

(fn ConstructionScript)

(fn DisplaySelection
  (Rendering|Components|Decal|SetDecalMaterial (Variables|Default|GetDecal) (Utilities|Array|Get(acopy) (Variables|Default|GetSymbols) (Variables|Default|GetValue))))
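; Trigger-driven Blueprint that moves a mesh between start and end positions as players enter and exit.
; BeginBehaviour puts the mesh at StartPos and sets the timeline play rate from Speed.
; PlayerEnter increments an activation count and plays the Moving timeline, lerping the mesh's relative location without sweep.
; PlayerExit decrements the count and reverses the timeline at zero, unless SingleUse is set.
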(event EventPlayerEnter
  (Math|Integer|IncrementInt (Variables|Default|GetActivated)
    (:%20%20
      (bind _time (Timeline|Moving Play)
        (:Update
          (Transformation|SetRelativeLocation (Variables|Default|GetMesh) (Math|Vector|Lerp(Vector) (Variables|Default|GetStartPos) (Variables|Default|GetEndPos) _time) false false))))))

(event EventPlayerExit
  (if (not (Variables|Default|GetSingleUse))
    (bind _result (Math|Integer|DecrementInt (Variables|Default|GetActivated))
      (:%20%20
        (if (== _result 0)
          (bind _time (Timeline|Moving Reverse)
            (:Update
              (Transformation|SetRelativeLocation (Variables|Default|GetMesh) (Math|Vector|Lerp(Vector) (Variables|Default|GetStartPos) (Variables|Default|GetEndPos) _time) false false))))))))

(fn ConstructionScript
  (|CallParentFunction))

(fn BeginBehaviour
  (Transformation|SetRelativeLocation (Variables|Default|GetMesh) (Variables|Default|GetStartPos) false false)
  (Components|Timeline|SetPlayRate (Variables|Default|GetMoving) (Variables|Default|GetSpeed)))
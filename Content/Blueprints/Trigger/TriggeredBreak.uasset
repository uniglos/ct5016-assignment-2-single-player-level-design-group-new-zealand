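; Trigger behaviour that swaps an intact object for a Geometry Collection and breaks it apart when the player enters.
; BeginBehaviour keeps the breakable object hidden, without collision or physics simulation.
; PlayerEnter hides the replaced object, reveals the breakable one, enables its physics and applies a configurable impulse at a set location to scatter it.
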(event EventPlayerEnter
  (bind _breakobject (Variables|Default|GetBreakObject))
  (bind _replaceobject (Variables|Default|GetReplaceObject))
  (bind _geometrycollectioncomponent (Variables|/Script/GeometryCollectionEngine.GeometryCollectionActor|GetGeometryCollectionComponent _breakobject))
  (Rendering|SetActorHiddenInGame _replaceobject true)
  (Collision|SetActorEnableCollision _replaceobject false)
  (Rendering|SetActorHiddenInGame _breakobject false)
  (Collision|SetActorEnableCollision _breakobject true)
  (Physics|SetSimulatePhysics _geometrycollectioncomponent true)
  (Physics|AddImpulseatLocation _geometrycollectioncomponent (Variables|Default|GetImpulseStrength) (Variables|Default|GetImpulsePosition) "None"))

(fn ConstructionScript
  (|CallParentFunction))

(fn BeginBehaviour
  (bind _breakobject (Variables|Default|GetBreakObject))
  (Rendering|SetActorHiddenInGame _breakobject true)
  (Collision|SetActorEnableCollision _breakobject false)
  (Physics|SetSimulatePhysics (Variables|/Script/GeometryCollectionEngine.GeometryCollectionActor|GetGeometryCollectionComponent _breakobject) false))
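; Trigger Blueprint that keeps an actor dormant until the player enters.
; BeginBehaviour switches off collision and tick on the referenced Actor.
; The PlayerEnter event switches both back on, with no logic here to deactivate it again afterwards.
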(event EventBeginPlay
  (|CallParentFunction) ; This node is disabled and will not be called.\nDrag off pins to build functionality.
)

(event Collision|EventActorBeginOverlap
  (params (OtherActor :type Actor%20Object%20Reference)))

(event EventTick
  (params (DeltaSeconds :type Float%20%28single-precision%29)))

(event EventPlayerEnter
  (bind _actor (Variables|Default|GetActor))
  (Collision|SetActorEnableCollision _actor true)
  (Actor|Tick|SetActorTickEnabled _actor true))

(fn ConstructionScript
  (|CallParentFunction))

(fn BeginBehaviour
  (bind _actor (Variables|Default|GetActor))
  (Collision|SetActorEnableCollision _actor false)
  (Actor|Tick|SetActorTickEnabled _actor))
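; TriggeredActor is a base actor that responds to a list of trigger objects.
; On BeginPlay it binds its player enter, player exit, any enter and any leave events to each entry in Triggers.
; It calls BeginBehaviour inside that loop, so it runs once per trigger rather than once overall.
; The four events and BeginBehaviour are empty hooks, apparently for child Blueprints to override.
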(event Custom|Player%20Enter)

(event Custom|Player%20Exit)

(event Custom|Any%20Enter)

(event Custom|Any%20Leave)

(event EventBeginPlay
  (for _array_element (Variables|Default|GetTriggers)
    (EventDispatchers|BindEventtoPlayerEnter _array_element (delegate Custom|Player%20Enter))
    (EventDispatchers|BindEventtoPlayerLeave _array_element (delegate Custom|Player%20Exit))
    (EventDispatchers|BindEventtoAnyEnter _array_element (delegate Custom|Any%20Enter))
    (EventDispatchers|BindEventtoAnyLeave _array_element (delegate Custom|Any%20Leave))
    (CallFunction|BeginBehaviour)))

(fn ConstructionScript)

(fn BeginBehaviour)
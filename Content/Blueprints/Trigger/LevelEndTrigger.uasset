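; LevelEndTrigger is a trigger actor that ends the level when BP_Player overlaps its Box component.
; On overlap it tells LevelTimer that the level is over, then branches on LevelTransition.
; When that flag is set it opens the level named by LevelName; otherwise it adds an EndWidget to the viewport and calls its GameOver.
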(event OnComponentBeginOverlap(Box)
  (params (OverlappedComponent :type Primitive%20Component%20Object%20Reference) (OtherActor :type Actor%20Object%20Reference) (OtherComp :type Primitive%20Component%20Object%20Reference) (OtherBodyIndex :type Integer) (bFromSweep :type Boolean) (SweepResult :type Hit%20Result%20Structure%20%28by%20ref%29))
  (Utilities|Casting|CastToBP_Player OtherActor)
  (Default|LevelOver (Variables|Default|GetLevelTimer))
  (if (Variables|Default|GetLevelTransition?)
    (Game|OpenLevel(byName) (Variables|Default|GetLevelName))
    (else
      (bind _returnvalue (UserInterface|CreateWidget (Variables|Default|GetEndWidget)))
      (UserInterface|Viewport|AddtoViewport _returnvalue 0)
      (bind _asend_widget (Utilities|Casting|CastToEndWidget _returnvalue))
      (Default|GameOver _asend_widget))))

(event EventBeginPlay)

(event Collision|EventActorBeginOverlap
  (params (OtherActor :type Actor%20Object%20Reference)))

(event EventTick
  (params (DeltaSeconds :type Float%20%28single-precision%29)))

(fn ConstructionScript)
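; A triggered light actor whose point light responds to actors entering and leaving it.
; An occupancy counter sets the light to its configured intensity when the first actor enters and to zero when the last leaves.
; Player enter and exit events switch the colour between a player colour and a general colour.
; The construction script calls its parent, then applies the general colour.
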(event EventPlayerEnter
  (Rendering|Components|Light|SetLightColor (Variables|Default|GetPointLight) (Variables|Default|GetPlayerColour) true))

(event EventPlayerExit
  (Rendering|Components|Light|SetLightColor (Variables|Default|GetPointLight) (Variables|Default|GetAllColour) true))

(event EventAnyEnter
  (bind _result (Math|Integer|IncrementInt (Variables|Default|GetActorsHere))
    (:%20%20
      (if (== _result 1)
        (Rendering|Components|Light|SetIntensity (Variables|Default|GetPointLight) (Variables|Default|GetIntensity))))))

(event EventAnyLeave
  (bind _result (Math|Integer|DecrementInt (Variables|Default|GetActorsHere))
    (:%20%20
      (if (== _result 0)
        (Rendering|Components|Light|SetIntensity (Variables|Default|GetPointLight) 0.0)))))

(fn ConstructionScript
  (|CallParentFunction)
  (Rendering|Components|Light|SetLightColor (Variables|Default|GetPointLight) (Variables|Default|GetAllColour) true))